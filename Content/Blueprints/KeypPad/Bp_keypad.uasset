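; Interactive world keypad that unlocks a linked Door when the player enters the correct code.
; Interact blends the view to the keypad and enables mouse clicks on its key components, which build an input string shown on screen.
; Enter compares it to CorrectCode, then either calls AccessGranted on the Door and exits, or briefly shows an invalid message and resets.
; CapsLock also exits, restoring the player's view and controls.
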(event OnBeginCursorOver(1_Key)
  (params (TouchedComponent :type Primitive%20Component%20Object%20Reference))
  ;[0.15 0.15 0.15 0.5] Button Presses
  (Development|PrintString "Hover"))

(event OnClicked(1_Key)
  (params (TouchedComponent :type Primitive%20Component%20Object%20Reference) (ButtonPressed :type Key%20Structure :default "None"))
  ;[0.15 0.15 0.15 0.5] Button Presses
  (Audio|PlaySound2D "/Game/Blueprints/KeypPad/ButtonPress.ButtonPress" 1.0 1.0 0.0 0 0)
  (bind _output_get (Variables|Default|SetInput (Utilities|String|Append (Variables|Default|GetInput) "1")))
  (Rendering|Components|TextRender|SetText (Variables|Default|GetCode) (Utilities|Text|ToText(String) _output_get))
  (Development|PrintString "bUTTON 1 PRESSED")
  (CallFunction|ShowScreen))

(event OnBeginCursorOver(6_Key)
  (params (TouchedComponent :type Primitive%20Component%20Object%20Reference))
  ;[0.15 0.15 0.15 0.5] Button Presses
  (Development|PrintString "Hover"))

(event OnClicked(6_Key)
  (params (TouchedComponent :type Primitive%20Component%20Object%20Reference) (ButtonPressed :type Key%20Structure :default "None"))
  ;[0.15 0.15 0.15 0.5] Button Presses
  (Audio|PlaySound2D "/Game/Blueprints/KeypPad/ButtonPress.ButtonPress" 1.0 1.0 0.0 0 0)
  (bind _output_get (Variables|Default|SetInput (Utilities|String|Append (Variables|Default|GetInput) "6")))
  (Rendering|Components|TextRender|SetText (Variables|Default|GetCode) (Utilities|Text|ToText(String) _output_get))
  (Development|PrintString "bUTTON 6 PRESSED")
  (CallFunction|ShowScreen))

(event OnBeginCursorOver(7_Key)
  (params (TouchedComponent :type Primitive%20Component%20Object%20Reference))
  ;[0.15 0.15 0.15 0.5] Button Presses
  (Development|PrintString "Hover"))

(event OnClicked(7_Key)
  (params (TouchedComponent :type Primitive%20Component%20Object%20Reference) (ButtonPressed :type Key%20Structure :default "None"))
  ;[0.15 0.15 0.15 0.5] Button Presses
  (Audio|PlaySound2D "/Game/Blueprints/KeypPad/ButtonPress.ButtonPress" 1.0 1.0 0.0 0 0)
  (bind _output_get (Variables|Default|SetInput (Utilities|String|Append (Variables|Default|GetInput) "7")))
  (Rendering|Components|TextRender|SetText (Variables|Default|GetCode) (Utilities|Text|ToText(String) _output_get))
  (Development|PrintString "bUTTON 7 PRESSED")
  (CallFunction|ShowScreen))

(event OnBeginCursorOver(8_Key)
  (params (TouchedComponent :type Primitive%20Component%20Object%20Reference))
  ;[0.15 0.15 0.15 0.5] Button Presses
  (Development|PrintString "Hover"))

(event OnClicked(8_Key)
  (params (TouchedComponent :type Primitive%20Component%20Object%20Reference) (ButtonPressed :type Key%20Structure :default "None"))
  ;[0.15 0.15 0.15 0.5] Button Presses
  (Audio|PlaySound2D "/Game/Blueprints/KeypPad/ButtonPress.ButtonPress" 1.0 1.0 0.0 0 0)
  (bind _output_get (Variables|Default|SetInput (Utilities|String|Append (Variables|Default|GetInput) "8")))
  (Rendering|Components|TextRender|SetText (Variables|Default|GetCode) (Utilities|Text|ToText(String) _output_get))
  (Development|PrintString "bUTTON 8 PRESSED")
  (CallFunction|ShowScreen))

(event OnBeginCursorOver(9_Key)
  (params (TouchedComponent :type Primitive%20Component%20Object%20Reference))
  ;[0.15 0.15 0.15 0.5] Button Presses
  (Development|PrintString "Hover"))

(event OnClicked(9_Key)
  (params (TouchedComponent :type Primitive%20Component%20Object%20Reference) (ButtonPressed :type Key%20Structure :default "None"))
  ;[0.15 0.15 0.15 0.5] Button Presses
  (Audio|PlaySound2D "/Game/Blueprints/KeypPad/ButtonPress.ButtonPress" 1.0 1.0 0.0 0 0)
  (bind _output_get (Variables|Default|SetInput (Utilities|String|Append (Variables|Default|GetInput) "9")))
  (Rendering|Components|TextRender|SetText (Variables|Default|GetCode) (Utilities|Text|ToText(String) _output_get))
  (Development|PrintString "bUTTON 9 PRESSED")
  (CallFunction|ShowScreen))

(event OnBeginCursorOver(0_Key)
  (params (TouchedComponent :type Primitive%20Component%20Object%20Reference))
  ;[0.15 0.15 0.15 0.5] Button Presses
  (Development|PrintString "Hover"))

(event OnClicked(0_Key)
  (params (TouchedComponent :type Primitive%20Component%20Object%20Reference) (ButtonPressed :type Key%20Structure :default "None"))
  ;[0.15 0.15 0.15 0.5] Button Presses
  (Audio|PlaySound2D "/Game/Blueprints/KeypPad/ButtonPress.ButtonPress" 1.0 1.0 0.0 0 0)
  (bind _output_get (Variables|Default|SetInput (Utilities|String|Append (Variables|Default|GetInput) "0")))
  (Rendering|Components|TextRender|SetText (Variables|Default|GetCode) (Utilities|Text|ToText(String) _output_get))
  (Development|PrintString "bUTTON 0 PRESSED")
  (CallFunction|ShowScreen))

(event OnBeginCursorOver(2_Key)
  (params (TouchedComponent :type Primitive%20Component%20Object%20Reference))
  ;[0.15 0.15 0.15 0.5] Button Presses
  (Development|PrintString "Hover"))

(event OnBeginCursorOver(Back_Key)
  (params (TouchedComponent :type Primitive%20Component%20Object%20Reference))
  ;[0.15 0.15 0.15 0.5] Button Presses
  (Development|PrintString "Hover"))

(event OnClicked(Back_Key)
  (params (TouchedComponent :type Primitive%20Component%20Object%20Reference) (ButtonPressed :type Key%20Structure :default "None"))
  ;[0.15 0.15 0.15 0.5] Button Presses
  (Audio|PlaySound2D "/Game/Blueprints/KeypPad/ButtonPress.ButtonPress" 1.0 1.0 0.0 0 0)
  (bind _output_get (Variables|Default|SetInput ""))
  (Rendering|Components|TextRender|SetText (Variables|Default|GetCode) (Utilities|Text|ToText(String) _output_get))
  (CallFunction|ShowScreen))

(event OnClicked(Enter_Key)
  (params (TouchedComponent :type Primitive%20Component%20Object%20Reference) (ButtonPressed :type Key%20Structure :default "None"))
  (bind _door (Variables|Default|GetDoor))
  (bind _textcode (Variables|Default|GetTextCode))
  ;[0.15 0.15 0.15 0.5] Button Presses
  (Audio|PlaySound2D "/Game/Blueprints/KeypPad/ButtonPress.ButtonPress" 1.0 1.0 0.0 0 0)
  (if (Utilities|Enum|Equal(Enum) (Variables|Default|GetInput) (Variables|Default|GetCorrectCode))
    (Development|SetHiddeninGame (Variables|Default|GetTextCorrect) false false)
    (Development|SetHiddeninGame (Variables|Default|GetTextCode) true false)
    (CallFunction|ShowScreen)
    (Development|PrintString (Utilities|GetDisplayName _door) true true "(R=1.000000,G=0.107935,B=0.000000,A=1.000000)")
    (Default|AccessGranted _door)
    (Appearance|SetColorandOpacity (Variables|Default|GetCode) (Variables|Default|GetIn%20Color%20and%20Opacity) :!class /Script/UMG.TextBlock)
    (Utilities|FlowControl|Delay 1.0)
    (bind _output_get (Variables|Default|SetInput ""))
    (Rendering|Components|TextRender|SetText (Variables|Default|GetCode) (Utilities|Text|ToText(String) _output_get))
    (CallFunction|ShowScreen)
    (CallFunction|ExView)
    (else
      (Development|SetHiddeninGame (Variables|Default|GetTextCode) true false)
      (Development|SetHiddeninGame (Variables|Default|GetTextInvalid) false false)
      (CallFunction|ShowScreen)
      (Utilities|FlowControl|Delay 2.0)
      (Development|SetHiddeninGame (Variables|Default|GetTextInvalid) true false)
      (Appearance|SetColorandOpacity (Variables|Default|GetCode) (Variables|Default|GetIn%20Color%20and%20Opacity_0) :!class /Script/UMG.TextBlock)
      (Utilities|FlowControl|Delay 1.2)
      (Appearance|SetColorandOpacity (Variables|Default|GetCode) (Variables|Default|GetIn%20Color%20and%20Opacity_1) :!class /Script/UMG.TextBlock)
      (bind _output_get_2 (Variables|Default|SetInput ""))
      (Rendering|Components|TextRender|SetText _textcode (Utilities|Text|ToText(String) _output_get_2))
      (Development|SetHiddeninGame _textcode false false)
      (CallFunction|ShowScreen))))

(event OnClicked(2_Key)
  (params (TouchedComponent :type Primitive%20Component%20Object%20Reference) (ButtonPressed :type Key%20Structure :default "None"))
  ;[0.15 0.15 0.15 0.5] Button Presses
  (Audio|PlaySound2D "/Game/Blueprints/KeypPad/ButtonPress.ButtonPress" 1.0 1.0 0.0 0 0)
  (bind _output_get (Variables|Default|SetInput (Utilities|String|Append (Variables|Default|GetInput) "2")))
  (Rendering|Components|TextRender|SetText (Variables|Default|GetCode) (Utilities|Text|ToText(String) _output_get))
  (Development|PrintString "bUTTON 2 PRESSED")
  (CallFunction|ShowScreen))

(event OnBeginCursorOver(Enter_Key)
  (params (TouchedComponent :type Primitive%20Component%20Object%20Reference))
  ;[0.15 0.15 0.15 0.5] Button Presses
  (Development|PrintString "Hover"))

(event OnBeginCursorOver(3_Key)
  (params (TouchedComponent :type Primitive%20Component%20Object%20Reference))
  ;[0.15 0.15 0.15 0.5] Button Presses
  (Development|PrintString "Hover"))

(event OnClicked(3_Key)
  (params (TouchedComponent :type Primitive%20Component%20Object%20Reference) (ButtonPressed :type Key%20Structure :default "None"))
  ;[0.15 0.15 0.15 0.5] Button Presses
  (Audio|PlaySound2D "/Game/Blueprints/KeypPad/ButtonPress.ButtonPress" 1.0 1.0 0.0 0 0)
  (bind _output_get (Variables|Default|SetInput (Utilities|String|Append (Variables|Default|GetInput) "3")))
  (Rendering|Components|TextRender|SetText (Variables|Default|GetCode) (Utilities|Text|ToText(String) _output_get))
  (Development|PrintString "bUTTON 3 PRESSED")
  (CallFunction|ShowScreen))

(event OnBeginCursorOver(4_Key)
  (params (TouchedComponent :type Primitive%20Component%20Object%20Reference))
  ;[0.15 0.15 0.15 0.5] Button Presses
  (Development|PrintString "Hover"))

(event OnClicked(4_Key)
  (params (TouchedComponent :type Primitive%20Component%20Object%20Reference) (ButtonPressed :type Key%20Structure :default "None"))
  ;[0.15 0.15 0.15 0.5] Button Presses
  (Audio|PlaySound2D "/Game/Blueprints/KeypPad/ButtonPress.ButtonPress" 1.0 1.0 0.0 0 0)
  (bind _output_get (Variables|Default|SetInput (Utilities|String|Append (Variables|Default|GetInput) "4")))
  (Rendering|Components|TextRender|SetText (Variables|Default|GetCode) (Utilities|Text|ToText(String) _output_get))
  (Development|PrintString "bUTTON 4 PRESSED")
  (CallFunction|ShowScreen))

(event OnBeginCursorOver(5_Key)
  (params (TouchedComponent :type Primitive%20Component%20Object%20Reference))
  ;[0.15 0.15 0.15 0.5] Button Presses
  (Development|PrintString "Hover"))

(event OnClicked(5_Key)
  (params (TouchedComponent :type Primitive%20Component%20Object%20Reference) (ButtonPressed :type Key%20Structure :default "None"))
  ;[0.15 0.15 0.15 0.5] Button Presses
  (Audio|PlaySound2D "/Game/Blueprints/KeypPad/ButtonPress.ButtonPress" 1.0 1.0 0.0 0 0)
  (bind _output_get (Variables|Default|SetInput (Utilities|String|Append (Variables|Default|GetInput) "5")))
  (Rendering|Components|TextRender|SetText (Variables|Default|GetCode) (Utilities|Text|ToText(String) _output_get))
  (Development|PrintString "bUTTON 5 PRESSED")
  (CallFunction|ShowScreen))

(event Custom|exView
  (bind _returnvalue (Game|GetPlayerController 0))
  (bind _output_get (Variables|Default|SetInput ""))
  (Rendering|Components|TextRender|SetText (Variables|Default|GetCode) (Utilities|Text|ToText(String) _output_get))
  (CallFunction|ShowScreen)
  (Game|Player|SetViewTargetwithBlend (Game|GetPlayerController 0) (Game|Player|GetPlayerPawn 0) 0.5 "VTBlend_Linear" 0.0 false)
  (Utilities|FlowControl|Delay 0.4)
  (Input|DisableInput _returnvalue)
  (Input|ResetIgnoreLookInput _returnvalue)
  (Variables|/Script/Engine.PlayerController|SetbShowMouseCursor _returnvalue false)
  (Variables|/Script/Engine.PlayerController|SetbEnableClickEvents _returnvalue false)
  (Variables|/Script/Engine.PlayerController|SetbEnableMouseOverEvents _returnvalue false)
  (Transformation|SetMobility (Variables|/Game/FirstPerson/Blueprints/BP_ZeroGChar.BP_ZeroGChar_C|GetCapsule (Variables|Default|GetAs%20BP%20Zero%20GChar)) "Movable")
  (Input|EnableInput (Game|Player|GetPlayerPawn 0) _returnvalue))

(event Custom|Show%20Screen
  (Rendering|Components|TextRender|SetText (Variables|Default|GetTextCode) (Utilities|Text|ToText(String) (Variables|Default|GetInput)))
  (Variables|Default|SetButtons (Utilities|Array|MakeArray (Variables|Default|Get1_Key) (Variables|Default|Get2_Key) (Variables|Default|Get3_Key) (Variables|Default|Get4_Key) (Variables|Default|Get5_Key) (Variables|Default|Get6_Key) (Variables|Default|Get7_Key) (Variables|Default|Get8_Key) (Variables|Default|Get9_Key) (Variables|Default|Get0_Key) (Variables|Default|GetBack_Key) (Variables|Default|GetEnter_Key))))

(event EventBeginPlay)

(event EventInteract
  (params (CharRef :type BP%20Zero%20G%20Char%20Object%20Reference))
  (bind _returnvalue (Game|GetPlayerController 0))
  (Input|SetIgnoreLookInput _returnvalue true)
  (Game|Player|SetViewTargetwithBlend (Game|GetPlayerController 0) self 0.5 "VTBlend_Linear" 0.0 false)
  (Variables|/Script/Engine.PlayerController|SetbEnableClickEvents _returnvalue true)
  (Variables|/Script/Engine.PlayerController|SetbEnableMouseOverEvents _returnvalue true)
  (Input|EnableInput _returnvalue)
  (Variables|/Script/Engine.PlayerController|SetbShowMouseCursor _returnvalue true)
  (bind _asbp_zero_gchar (Utilities|Casting|CastToBP_ZeroGChar (Game|Player|GetPlayerPawn 0)))
  (Variables|Default|SetAs%20BP%20Zero%20GChar _asbp_zero_gchar))

(event Input|KeyboardEvents|CapsLock
  (params (Key :type Key%20Structure :default "None"))
  (:Pressed
    (CallFunction|ExView)))

(fn ConstructionScript)