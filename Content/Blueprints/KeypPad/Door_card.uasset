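; Door actor, apparently card-locked, that swings open when interacted with while its CanUnlock flag is true.
; Interact triggers AccessGranted, which plays the OpenDoor timeline to lerp the Door component's relative rotation through a quarter turn.
; BeginPlay caches the player pawn as BP_ZeroGChar, though nothing here uses it.
; This graph only reads CanUnlock and has no closing logic.
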(event Custom|Access%20granted
  (bind _open (Timeline|Open%20Door Play)
    (:Update
      (Transformation|SetRelativeRotation (Variables|Default|GetDoor) (Math|Rotator|Lerp(Rotator) "0, 0, 0" "0.000000,-90.000000,0.000000" _open) false false))))

(event Collision|EventActorBeginOverlap
  (params (OtherActor :type Actor%20Object%20Reference)))

(event EventTick
  (params (DeltaSeconds :type Float%20%28single-precision%29)))

(event EventBeginPlay
  (bind _asbp_zero_gchar (Utilities|Casting|CastToBP_ZeroGChar (Game|Player|GetPlayerPawn 0)))
  (Variables|Default|SetPlayer _asbp_zero_gchar))

(event EventInteract
  (params (CharRef :type BP%20Zero%20G%20Char%20Object%20Reference))
  (if (Variables|Default|GetCanUnlock)
    (CallFunction|AccessGranted)))

(fn ConstructionScript)