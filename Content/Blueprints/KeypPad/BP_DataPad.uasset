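; BP_DataPad is an interactable data pad that shows a text screen and marks itself with a flashing light.
; On BeginPlay it sets its spotlight color, caches the intensity, and plays a timeline that scales that intensity to make it flash.
; Interact creates a WB_DataPadScreen widget, fills it with OnScreenText, adds it to the viewport and passes the character reference on to the widget's Interact.
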(event EventBeginPlay
  ;[0.15 0.15 0.15 0.5] Flahing Light ON object
  (Rendering|Components|Light|SetLightColor (Variables|Default|GetSpotLight) (Variables|Default|GetNew%20Light%20Color) true)
  (Variables|Default|SetLightIntesity (Variables|/Script/Engine.LightComponentBase|GetIntensity (Variables|Default|GetSpotLight)))
  (bind _lighting_off (Timeline|Flahing Play)
    (:Update
      (Rendering|Components|Light|SetIntensity (Variables|Default|GetSpotLight) (* (Variables|Default|GetLightIntesity) _lighting_off)))))

(event EventInteract
  (params (CharRef :type BP%20Zero%20G%20Char%20Object%20Reference))
  ;[0.15 0.15 0.15 0.5] Adds Text
  (bind _returnvalue (UserInterface|CreateWidget "/Game/HUD_UI/WB_DataPadScreen.WB_DataPadScreen_C" (Game|GetPlayerController 0)))
  (Rendering|Components|TextRender|SetText (Variables|/Game/HUD_UI/WB_DataPadScreen.WB_DataPadScreen_C|GetText _returnvalue) (Variables|Default|GetOn%20Screen%20Text))
  (UserInterface|Viewport|AddtoViewport _returnvalue 0)
  (Default|Interact _returnvalue CharRef))

(fn ConstructionScript)