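; Keypad code actor that shows a WB_CodeText widget while a BP_ZeroGChar is inside its box trigger.
; Beginning overlap enables input for player 0 and creates the widget on screen, while ending overlap disables input and removes it.
; Pressing E while input is enabled destroys the actor and removes the widget, without storing or passing on any code.
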(event OnComponentBeginOverlap(Box)
  (params (OverlappedComponent :type Primitive%20Component%20Object%20Reference) (OtherActor :type Actor%20Object%20Reference) (OtherComp :type Primitive%20Component%20Object%20Reference) (OtherBodyIndex :type Integer) (bFromSweep :type Boolean) (SweepResult :type Hit%20Result%20Structure%20%28by%20ref%29))
  (bind _returnvalue (Game|GetPlayerController 0))
  (Utilities|Casting|CastToBP_ZeroGChar OtherActor)
  (Input|EnableInput _returnvalue)
  (bind _returnvalue_2 (UserInterface|CreateWidget "/Game/HUD_UI/WB_CodeText.WB_CodeText_C" _returnvalue))
  (bind _output_get (Variables|Default|SetWBTextCode _returnvalue_2))
  (UserInterface|Viewport|AddtoViewport _output_get 0))

(event OnComponentEndOverlap(Box)
  (params (OverlappedComponent :type Primitive%20Component%20Object%20Reference) (OtherActor :type Actor%20Object%20Reference) (OtherComp :type Primitive%20Component%20Object%20Reference) (OtherBodyIndex :type Integer))
  (Utilities|Casting|CastToBP_ZeroGChar OtherActor)
  (Input|DisableInput (Game|GetPlayerController 0))
  (Widget|RemovefromParent (Variables|Default|GetWBTextCode)))

(event Input|KeyboardEvents|E
  (params (Key :type Key%20Structure :default "None"))
  (:Pressed
    (Actor|DestroyActor)
    (Widget|RemovefromParent (Variables|Default|GetWBTextCode))))

(fn ConstructionScript)