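; Interactive keypad actor where the player clicks digits to enter a code that unlocks a door.
; Interact blends the camera to the keypad and enables mouse clicks; CapsLock blends back and restores BP_ZeroGChar control.
; Digit buttons append to an input string mirrored on two text displays, and Clear empties it.
; Enter compares it to CorrectCode, calling AccessGranted on the Door found by class, or briefly showing an error.
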(event OnBeginCursorOver(button_2)
  (params (TouchedComponent :type Primitive%20Component%20Object%20Reference))
  ;[0.15 0.15 0.15 0.5] Button Presses
  (Development|PrintString "Hover"))

(event OnClicked(button_2)
  (params (TouchedComponent :type Primitive%20Component%20Object%20Reference) (ButtonPressed :type Key%20Structure :default "None"))
  ;[0.15 0.15 0.15 0.5] Button Presses
  (Audio|PlaySound2D "/Game/Blueprints/ButtonPress.ButtonPress" 1.0 1.0 0.0 0 0)
  (bind _output_get (Variables|Default|SetInput (Utilities|String|Append (Variables|Default|GetInput) "2")))
  (Rendering|Components|TextRender|SetText (Variables|Default|GetCode) (Utilities|Text|ToText(String) _output_get))
  (Development|PrintString "bUTTON 2 PRESSED")
  (CallFunction|ShowScreen))

(event OnBeginCursorOver(button_6)
  (params (TouchedComponent :type Primitive%20Component%20Object%20Reference))
  ;[0.15 0.15 0.15 0.5] Button Presses
  (Development|PrintString "Hover"))

(event OnClicked(button_6)
  (params (TouchedComponent :type Primitive%20Component%20Object%20Reference) (ButtonPressed :type Key%20Structure :default "None"))
  ;[0.15 0.15 0.15 0.5] Button Presses
  (Audio|PlaySound2D "/Game/Blueprints/ButtonPress.ButtonPress" 1.0 1.0 0.0 0 0)
  (bind _output_get (Variables|Default|SetInput (Utilities|String|Append (Variables|Default|GetInput) "6")))
  (Rendering|Components|TextRender|SetText (Variables|Default|GetCode) (Utilities|Text|ToText(String) _output_get))
  (Development|PrintString "bUTTON 6 PRESSED")
  (CallFunction|ShowScreen))

(event OnBeginCursorOver(button_7)
  (params (TouchedComponent :type Primitive%20Component%20Object%20Reference))
  ;[0.15 0.15 0.15 0.5] Button Presses
  (Development|PrintString "Hover"))

(event OnClicked(button_7)
  (params (TouchedComponent :type Primitive%20Component%20Object%20Reference) (ButtonPressed :type Key%20Structure :default "None"))
  ;[0.15 0.15 0.15 0.5] Button Presses
  (Audio|PlaySound2D "/Game/Blueprints/ButtonPress.ButtonPress" 1.0 1.0 0.0 0 0)
  (bind _output_get (Variables|Default|SetInput (Utilities|String|Append (Variables|Default|GetInput) "7")))
  (Rendering|Components|TextRender|SetText (Variables|Default|GetCode) (Utilities|Text|ToText(String) _output_get))
  (Development|PrintString "bUTTON 7 PRESSED")
  (CallFunction|ShowScreen))

(event OnBeginCursorOver(button_8)
  (params (TouchedComponent :type Primitive%20Component%20Object%20Reference))
  ;[0.15 0.15 0.15 0.5] Button Presses
  (Development|PrintString "Hover"))

(event OnClicked(button_8)
  (params (TouchedComponent :type Primitive%20Component%20Object%20Reference) (ButtonPressed :type Key%20Structure :default "None"))
  ;[0.15 0.15 0.15 0.5] Button Presses
  (Audio|PlaySound2D "/Game/Blueprints/ButtonPress.ButtonPress" 1.0 1.0 0.0 0 0)
  (bind _output_get (Variables|Default|SetInput (Utilities|String|Append (Variables|Default|GetInput) "8")))
  (Rendering|Components|TextRender|SetText (Variables|Default|GetCode) (Utilities|Text|ToText(String) _output_get))
  (Development|PrintString "bUTTON 8 PRESSED")
  (CallFunction|ShowScreen))

(event OnBeginCursorOver(button_9)
  (params (TouchedComponent :type Primitive%20Component%20Object%20Reference))
  ;[0.15 0.15 0.15 0.5] Button Presses
  (Development|PrintString "Hover"))

(event OnClicked(button_9)
  (params (TouchedComponent :type Primitive%20Component%20Object%20Reference) (ButtonPressed :type Key%20Structure :default "None"))
  ;[0.15 0.15 0.15 0.5] Button Presses
  (Audio|PlaySound2D "/Game/Blueprints/ButtonPress.ButtonPress" 1.0 1.0 0.0 0 0)
  (bind _output_get (Variables|Default|SetInput (Utilities|String|Append (Variables|Default|GetInput) "9")))
  (Rendering|Components|TextRender|SetText (Variables|Default|GetCode) (Utilities|Text|ToText(String) _output_get))
  (Development|PrintString "bUTTON 9 PRESSED")
  (CallFunction|ShowScreen))

(event OnBeginCursorOver(button_0)
  (params (TouchedComponent :type Primitive%20Component%20Object%20Reference))
  ;[0.15 0.15 0.15 0.5] Button Presses
  (Development|PrintString "Hover"))

(event OnClicked(button_0)
  (params (TouchedComponent :type Primitive%20Component%20Object%20Reference) (ButtonPressed :type Key%20Structure :default "None"))
  ;[0.15 0.15 0.15 0.5] Button Presses
  (Audio|PlaySound2D "/Game/Blueprints/ButtonPress.ButtonPress" 1.0 1.0 0.0 0 0)
  (bind _output_get (Variables|Default|SetInput (Utilities|String|Append (Variables|Default|GetInput) "0")))
  (Rendering|Components|TextRender|SetText (Variables|Default|GetCode) (Utilities|Text|ToText(String) _output_get))
  (Development|PrintString "bUTTON 0 PRESSED")
  (CallFunction|ShowScreen))

(event OnBeginCursorOver(button_1)
  (params (TouchedComponent :type Primitive%20Component%20Object%20Reference))
  ;[0.15 0.15 0.15 0.5] Button Presses
  (Development|PrintString "Hover"))

(event OnBeginCursorOver(Clear)
  (params (TouchedComponent :type Primitive%20Component%20Object%20Reference))
  ;[0.15 0.15 0.15 0.5] Button Presses
  (Development|PrintString "Hover"))

(event OnClicked(Clear)
  (params (TouchedComponent :type Primitive%20Component%20Object%20Reference) (ButtonPressed :type Key%20Structure :default "None"))
  ;[0.15 0.15 0.15 0.5] Button Presses
  (Audio|PlaySound2D "/Game/Blueprints/ButtonPress.ButtonPress" 1.0 1.0 0.0 0 0)
  (bind _output_get (Variables|Default|SetInput ""))
  (Rendering|Components|TextRender|SetText (Variables|Default|GetCode) (Utilities|Text|ToText(String) _output_get))
  (CallFunction|ShowScreen))

(event OnBeginCursorOver(Enter)
  (params (TouchedComponent :type Primitive%20Component%20Object%20Reference))
  ;[0.15 0.15 0.15 0.5] Button Presses
  (Development|PrintString "Hover"))

(event OnClicked(Enter)
  (params (TouchedComponent :type Primitive%20Component%20Object%20Reference) (ButtonPressed :type Key%20Structure :default "None"))
  ;[0.15 0.15 0.15 0.5] Button Presses
  (Audio|PlaySound2D "/Game/Blueprints/ButtonPress.ButtonPress" 1.0 1.0 0.0 0 0)
  (if (Utilities|Enum|Equal(Enum) (Variables|Default|GetInput) (Variables|Default|GetCorrectCode))
    (bind _returnvalue (Actor|GetActorOfClass "/Game/Blueprints/Door.Door_C"))
    (Default|AccessGranted _returnvalue)
    (Appearance|SetColorandOpacity (Variables|Default|GetCode) (Variables|Default|GetIn%20Color%20and%20Opacity) :!class /Script/UMG.TextBlock)
    (Utilities|FlowControl|Delay 0.4)
    (else
      (Rendering|Components|TextRender|SetText (Variables|Default|GetCode) "You're Wrong")
      (Appearance|SetColorandOpacity (Variables|Default|GetCode) (Variables|Default|GetIn%20Color%20and%20Opacity_0) :!class /Script/UMG.TextBlock)
      (Utilities|FlowControl|Delay 1.2)
      (Appearance|SetColorandOpacity (Variables|Default|GetCode) (Variables|Default|GetIn%20Color%20and%20Opacity_1) :!class /Script/UMG.TextBlock)
      (bind _output_get (Variables|Default|SetInput ""))
      (Rendering|Components|TextRender|SetText (Variables|Default|GetCode) (Utilities|Text|ToText(String) _output_get)))))

(event OnClicked(button_1)
  (params (TouchedComponent :type Primitive%20Component%20Object%20Reference) (ButtonPressed :type Key%20Structure :default "None"))
  ;[0.15 0.15 0.15 0.5] Button Presses
  (Audio|PlaySound2D "/Game/Blueprints/ButtonPress.ButtonPress" 1.0 1.0 0.0 0 0)
  (bind _output_get (Variables|Default|SetInput (Utilities|String|Append (Variables|Default|GetInput) "1")))
  (Rendering|Components|TextRender|SetText (Variables|Default|GetCode) (Utilities|Text|ToText(String) _output_get))
  (Development|PrintString "bUTTON 1 PRESSED")
  (CallFunction|ShowScreen))

(event OnBeginCursorOver(button_3)
  (params (TouchedComponent :type Primitive%20Component%20Object%20Reference))
  ;[0.15 0.15 0.15 0.5] Button Presses
  (Development|PrintString "Hover"))

(event OnClicked(button_3)
  (params (TouchedComponent :type Primitive%20Component%20Object%20Reference) (ButtonPressed :type Key%20Structure :default "None"))
  ;[0.15 0.15 0.15 0.5] Button Presses
  (Audio|PlaySound2D "/Game/Blueprints/ButtonPress.ButtonPress" 1.0 1.0 0.0 0 0)
  (bind _output_get (Variables|Default|SetInput (Utilities|String|Append (Variables|Default|GetInput) "3")))
  (Rendering|Components|TextRender|SetText (Variables|Default|GetCode) (Utilities|Text|ToText(String) _output_get))
  (Development|PrintString "bUTTON 3 PRESSED")
  (CallFunction|ShowScreen))

(event OnBeginCursorOver(button_4)
  (params (TouchedComponent :type Primitive%20Component%20Object%20Reference))
  ;[0.15 0.15 0.15 0.5] Button Presses
  (Development|PrintString "Hover"))

(event OnClicked(button_4)
  (params (TouchedComponent :type Primitive%20Component%20Object%20Reference) (ButtonPressed :type Key%20Structure :default "None"))
  ;[0.15 0.15 0.15 0.5] Button Presses
  (Audio|PlaySound2D "/Game/Blueprints/ButtonPress.ButtonPress" 1.0 1.0 0.0 0 0)
  (bind _output_get (Variables|Default|SetInput (Utilities|String|Append (Variables|Default|GetInput) "4")))
  (Rendering|Components|TextRender|SetText (Variables|Default|GetCode) (Utilities|Text|ToText(String) _output_get))
  (Development|PrintString "bUTTON 4 PRESSED")
  (CallFunction|ShowScreen))

(event OnBeginCursorOver(button_5)
  (params (TouchedComponent :type Primitive%20Component%20Object%20Reference))
  ;[0.15 0.15 0.15 0.5] Button Presses
  (Development|PrintString "Hover"))

(event OnClicked(button_5)
  (params (TouchedComponent :type Primitive%20Component%20Object%20Reference) (ButtonPressed :type Key%20Structure :default "None"))
  ;[0.15 0.15 0.15 0.5] Button Presses
  (Audio|PlaySound2D "/Game/Blueprints/ButtonPress.ButtonPress" 1.0 1.0 0.0 0 0)
  (bind _output_get (Variables|Default|SetInput (Utilities|String|Append (Variables|Default|GetInput) "5")))
  (Rendering|Components|TextRender|SetText (Variables|Default|GetCode) (Utilities|Text|ToText(String) _output_get))
  (Development|PrintString "bUTTON 5 PRESSED")
  (CallFunction|ShowScreen))

(event Custom|Enter%20Code)

(event Custom|exView
  (bind _returnvalue (Game|GetPlayerController 0))
  (Game|Player|SetViewTargetwithBlend (Game|GetPlayerController 0) (Game|Player|GetPlayerPawn 0) 0.5 "VTBlend_Linear" 0.0 false)
  (Utilities|FlowControl|Delay 0.4)
  (Input|DisableInput _returnvalue)
  (Input|ResetIgnoreLookInput _returnvalue)
  (Variables|/Script/Engine.PlayerController|SetbShowMouseCursor _returnvalue false)
  (Variables|/Script/Engine.PlayerController|SetbEnableClickEvents _returnvalue false)
  (Variables|/Script/Engine.PlayerController|SetbEnableMouseOverEvents _returnvalue false)
  (Transformation|SetMobility (Variables|/Game/FirstPerson/Blueprints/BP_ZeroGChar.BP_ZeroGChar_C|GetCapsule (Variables|Default|GetAs%20BP%20Zero%20GChar)) "Movable")
  (Input|EnableInput (Game|Player|GetPlayerPawn 0) _returnvalue))

(event Custom|Show%20Screen
  (bind _code_screen (Variables|Default|GetCode_screen))
  (Rendering|Components|TextRender|SetText _code_screen (Utilities|Text|ToText(String) (Variables|Default|GetInput)))
  (Rendering|Components|TextRender|SetTextRenderColor _code_screen (Math|Color|MakeColor 200 200 200 255))
  (Variables|Default|SetButtons (Utilities|Array|MakeArray (Variables|Default|Getbutton_1) (Variables|Default|Getbutton_2) (Variables|Default|Getbutton_3) (Variables|Default|Getbutton_4) (Variables|Default|Getbutton_5) (Variables|Default|Getbutton_6) (Variables|Default|Getbutton_7) (Variables|Default|Getbutton_8) (Variables|Default|Getbutton_9) (Variables|Default|Getbutton_0))))

(event EventBeginPlay)

(event EventInteract
  (params (CharRef :type BP%20Zero%20G%20Char%20Object%20Reference))
  (bind _returnvalue (Game|GetPlayerController 0))
  (Input|SetIgnoreLookInput _returnvalue true)
  (Game|Player|SetViewTargetwithBlend (Game|GetPlayerController 0) self 0.5 "VTBlend_Linear" 0.0 false)
  (Variables|/Script/Engine.PlayerController|SetbEnableClickEvents _returnvalue true)
  (Variables|/Script/Engine.PlayerController|SetbEnableMouseOverEvents _returnvalue true)
  (Input|EnableInput _returnvalue)
  (Variables|/Script/Engine.PlayerController|SetbShowMouseCursor _returnvalue true)
  (bind _asbp_zero_gchar (Utilities|Casting|CastToBP_ZeroGChar (Game|Player|GetPlayerPawn 0)))
  (Variables|Default|SetAs%20BP%20Zero%20GChar _asbp_zero_gchar))

(event Input|KeyboardEvents|CapsLock
  (params (Key :type Key%20Structure :default "None"))
  (:Pressed
    (CallFunction|ExView)))

(fn ConstructionScript)