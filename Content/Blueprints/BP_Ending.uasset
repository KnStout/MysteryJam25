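; Trigger-box actor that plays a sequence of dialogue lines when the player overlaps it, optionally serving as an ending.
; A one-shot overlap, consumed before the player check, creates the WB_Dialogue widget and binds its line-finished dispatcher to Text.
; Text feeds lines in order after a delay, chaining through that callback.
; After the last line, ending dialogue displays end options with UI-only mouse input; otherwise the widget is removed after a delay.
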(event OnComponentBeginOverlap(Box)
  (params (OverlappedComponent :type Primitive%20Component%20Object%20Reference) (OtherActor :type Actor%20Object%20Reference) (OtherComp :type Primitive%20Component%20Object%20Reference) (OtherBodyIndex :type Integer) (bFromSweep :type Boolean) (SweepResult :type Hit%20Result%20Structure%20%28by%20ref%29))
  (bind _returnvalue (Game|GetPlayerController 0))
  (Utilities|FlowControl|DoOnce false
    (:Completed
      (if (== OtherActor (Game|Player|GetPlayerPawn 0))
        (Utilities|IsValid (Variables|Default|GetWB_Dialog)
          (:Is%20Valid
            _)
          (:Is%20Not%20Valid
            (bind _returnvalue_2 (UserInterface|CreateWidget "/Game/HUD_UI/WB_Dialogue.WB_Dialogue_C" (Game|GetPlayerController 0)))
            (bind _output_get (Variables|Default|SetWB_Dialog _returnvalue_2))))
        (if (Variables|Default|GetIsEndingDialogue)
          (Input|SetInputModeUIOnly _returnvalue (Variables|Default|GetWB_Dialog) "DoNotLock" true)
          (Variables|/Script/Engine.PlayerController|SetbShowMouseCursor _returnvalue true)
          (Variables|/Script/Engine.PlayerController|SetbEnableMouseOverEvents _returnvalue true)
          (Variables|/Script/Engine.PlayerController|SetbEnableClickEvents _returnvalue true))
        (EventDispatchers|AssignOndialogueLineFinished _output_get (delegate Custom|Text))
        (UserInterface|Viewport|AddtoViewport (Variables|Default|GetWB_Dialog) 0)
        (CallFunction|Text)))))

(event Custom|Text
  (bind _dialoge (Variables|Default|GetDialoge))
  (bind _wb_dialog (Variables|Default|GetWB_Dialog))
  (if (== (Variables|Default|GetCurrentDialog) 0)
    _
    (else
      (Utilities|FlowControl|Delay (Variables|Default|GetDelay%20For%20New%20Line))))
  (Default|IncomingSpeach (Variables|Default|GetWB_Dialog) (Utilities|Array|Get(acopy) _dialoge (Variables|Default|GetCurrentDialog)) (Variables|Default|GetTextSpeed) false)
  (bind _output_get (Variables|Default|SetCurrentDialog (+ (Variables|Default|GetCurrentDialog) 1)))
  (if (>= _output_get (Utilities|Array|Length _dialoge))
    (if (Variables|Default|GetIsEndingDialogue)
      (Default|DisplayEndOptions _wb_dialog)
      (else
        (Utilities|FlowControl|Delay (Variables|Default|Getdelay%20for%20removing))
        (Widget|RemovefromParent _wb_dialog)))))

(fn ConstructionScript)